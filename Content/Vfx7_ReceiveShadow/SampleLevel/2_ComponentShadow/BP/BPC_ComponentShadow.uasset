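; Actor component that fakes received directional-light shadow on its owner's meshes and Cascade particles.
; BeginPlay caches the first directional light's direction and the owner's components, then updates either every tick or just once.
; UpdateShadow line-traces from the actor toward the light on Visibility, converting occlusion into an instant or interpolated shadow rate.
; That rate drives the "ComponentShadow" material scalar, using dynamic material instances for particles.
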(event `self.ReceiveBeginPlay`
  (bind _output_get (set `self.OwnerActor` (`self.GetOwner`)))
  (`/Engine/EditorBlueprintResources/StandardMacros.IsValid` _output_get
    (:`Is Valid`
      ;[1 1 1] ディレクショナルライトの方向を取得
      ; （本来はGetAllActorsOfClass使わず外部から設定するのが良いと思います）
      (bind _outactors (`GameplayStatics.GetAllActorsOfClass` "/Script/Engine.DirectionalLight"))
      (if (`KismetArrayLibrary.Array_IsValidIndex` _outactors)
        (set `self.LightVector` (* (`Actor.GetActorForwardVector` (`|GetArrayItem` _outactors)) -1.0))
        ;[1 1 1] このComponentがくっついているActorの操作するメッシュ、パーティクルのリストを取得
        (set `self.MeshComponents` (`Actor.K2_GetComponentsByClass` (`self.OwnerActor`) "/Script/Engine.MeshComponent"))
        (set `self.ParticleComponents` (`Actor.K2_GetComponentsByClass` (`self.OwnerActor`) "/Script/Engine.ParticleSystemComponent"))
        ;[1 1 1] 一つ以上あれば処理有効
        (if (or (> (`KismetArrayLibrary.Array_Length` (`self.MeshComponents`)) 0) (> (`KismetArrayLibrary.Array_Length` (`self.ParticleComponents`)) 0))
          (set `self.Valid` true)
          (if (`self.AlwaysCheck`)
            ;[1 1 1] 毎フレームチェックする
            (`self.SetComponentTickEnabled` true)
            (else
              ;[1 1 1] 初回の一回だけチェックする
              (`self.SetComponentTickEnabled` false)
              (`self.UpdateShadow` 1.0))))))))

(event `self.ReceiveTick`
  (params (DeltaSeconds :type "Float (single-precision)"))
  (`self.UpdateShadow` DeltaSeconds))

(fn `UpdateShadow`
  (params (DeltaSeconds :type "Float (double-precision)"))
  (locals (NowLocation :type "Vector Structure" :default (0.0 0.0 0.0)) (TraceShadowRate :type "Float (double-precision)" :default 0.0) (NumMaterial :type Integer :default 0) (Particle :type "ParticleSystemComponent Object Reference") (InShadow :type Boolean :default false))
  (bind _returnvalue (* (`local.DeltaSeconds`) 5.0))
  (if (`self.Valid`)
    ;[1 1 1] Actorの座標
    (set `local.NowLocation` (`Actor.K2_GetActorLocation` (`self.OwnerActor`)))
    ;[1 1 1] Actorの位置からライト方向に遮蔽物が有るか
    (bind (_outhit _returnvalue_2) (`KismetSystemLibrary.LineTraceSingle` (+ (`local.NowLocation`) (* (`self.LightVector`) 30.0)) (+ (`local.NowLocation`) (* (`self.LightVector`) (`self.TraceLength`))) "TraceTypeQuery1" false (`|MakeArray` (`self.OwnerActor`))))
    (set `local.InShadow` _returnvalue_2)
    (if (`self.Interpolate`)
      (set `self.ShadowRate` (`KismetMathLibrary.FClamp` (+ (`self.ShadowRate`) (`KismetMathLibrary.SelectFloat` _returnvalue (* _returnvalue -1.0) (`local.InShadow`)))))
      (else
        (set `self.ShadowRate` (`KismetMathLibrary.SelectFloat` 1.0 0.0 (`local.InShadow`)))))
    ;[1 1 1] 対象のメッシュとパーティクルに影の具合を設定
    (for _array_element (`self.MeshComponents`)
      (`MeshComponent.SetScalarParameterValueOnMaterials` _array_element "ComponentShadow" (`self.ShadowRate`)))
    (for _array_element_2 (`self.ParticleComponents`)
      (bind _output_get (set `local.Particle` _array_element_2))
      (bind _output_get_2 (set `local.NumMaterial` (`PrimitiveComponent.GetNumMaterials` _output_get)))
      (for _index (range _output_get_2)
        (bind _returnvalue_3 (`PrimitiveComponent.CreateDynamicMaterialInstance` (`local.Particle`) _index null "None"))
        (`MaterialInstanceDynamic.SetScalarParameterValue` _returnvalue_3 "ComponentShadow" (`self.ShadowRate`))))))