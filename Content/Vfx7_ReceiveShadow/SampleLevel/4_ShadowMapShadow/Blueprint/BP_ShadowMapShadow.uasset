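; BP_ShadowMapShadow is a sample actor that sets up a custom shadow map capture from the directional light's view.
; On BeginPlay it finds the first DirectionalLight and moves itself far back along the light's direction, matching its rotation.
; It writes the capture location and light view axes to MPC_ShadowMapShadow for materials.
; Its SceneCaptureComponent2D then captures once, or every frame if EveryFrameCapture is set.
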(event `self.ReceiveBeginPlay`
  ;[1 1 1] ライトの方向を取得する
  ; （本来はGetAllActorsOfClassを使わずに外から設定する方が良い
  (bind _outactors (`GameplayStatics.GetAllActorsOfClass` "/Script/Engine.DirectionalLight"))
  (if (> (`KismetArrayLibrary.Array_Length` _outactors) 0)
    (`self.SetupCapture` (`|GetArrayItem` _outactors))))

(fn `SetupCapture`
  (params (DirectionalLight :type "DirectionalLight Object Reference"))
  (locals (CaptureTransform :type "Transform Structure"))
  (bind _directionallight (`local.DirectionalLight`))
  (bind _rotation (.rotation (`local.CaptureTransform`)))
  (`/Engine/EditorBlueprintResources/StandardMacros.IsValid` DirectionalLight
    (:`Is Valid`
      ;[1 1 1] ライトの位置にActorを移動する
      (bind _output_get (set `local.CaptureTransform` (`KismetMathLibrary.MakeTransform` (* (`self.GetActorForwardVector` _directionallight) -10000.0) (`self.K2_GetActorRotation` _directionallight))))
      (`self.K2_SetActorTransform` _output_get false true)
      ;[1 1 1] ライトの配置情報をマテリアルに設定する
      (`KismetMaterialLibrary.SetVectorParameterValue` "/Game/Vfx7_ReceiveShadow/SampleLevel/4_ShadowMapShadow/Materials/MPC_ShadowMapShadow.MPC_ShadowMapShadow" "CaptureLocation" (`KismetMathLibrary.Conv_VectorToLinearColor` (.location (`local.CaptureTransform`))))
      (`KismetMaterialLibrary.SetVectorParameterValue` "/Game/Vfx7_ReceiveShadow/SampleLevel/4_ShadowMapShadow/Materials/MPC_ShadowMapShadow.MPC_ShadowMapShadow" "LightViewMatrixPlaneX" (`KismetMathLibrary.Conv_VectorToLinearColor` (`KismetMathLibrary.GetRightVector` _rotation)))
      (`KismetMaterialLibrary.SetVectorParameterValue` "/Game/Vfx7_ReceiveShadow/SampleLevel/4_ShadowMapShadow/Materials/MPC_ShadowMapShadow.MPC_ShadowMapShadow" "LightViewMatrixPlaneY" (`KismetMathLibrary.Conv_VectorToLinearColor` (`KismetMathLibrary.GetUpVector` _rotation)))
      (`KismetMaterialLibrary.SetVectorParameterValue` "/Game/Vfx7_ReceiveShadow/SampleLevel/4_ShadowMapShadow/Materials/MPC_ShadowMapShadow.MPC_ShadowMapShadow" "LightViewMatrixPlaneZ" (`KismetMathLibrary.Conv_VectorToLinearColor` (`KismetMathLibrary.GetForwardVector` _rotation)))
      (if (`self.EveryFrameCapture`)
        ;[1 1 1] 毎フレームキャプチャーする
        (set `SceneCaptureComponent.bCaptureEveryFrame` (`self.EveryFrameCapture`) (`self.SceneCaptureComponent2D`))
        (else
          ;[1 1 1] 初回だけキャプチャーする
          (`SceneCaptureComponent2D.CaptureScene` (`self.SceneCaptureComponent2D`)))))))

(fn `UserConstructionScript`)